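; Game mode base Blueprint with two events that lay out a centered grid of map tiles from a flattened list.
; GenerateLevelActors spawns tile actor classes with an extra X offset, while GenerateLevel creates uniquely named streaming-level instances set to load visibly and block on load.
; Both space tiles by SublevelSize and log progress.
; Random rotation goes through RotationFromXVector on a Y-only vector, yielding only 0 or 90 degree yaw.
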(event EventBeginPlay)

(event EventTick
  (params (DeltaSeconds :type Float%20%28single-precision%29)))

(event EventGenerateLevelActors
  (params (LevelList :type Array%20of%20Actor%20Class%20References) (MapTileCountX :type Integer) (MapTileCountY :type Integer))
  (bind _sublevelsize (Variables|Default|GetSublevelSize))
  (Class|VisualLoggerKismetLibrary|LogText "Executing generate level.." "Blueprint Log")
  (for _index (range 0 MapTileCountX)
    (for _index_2 (range 0 MapTileCountY)
      (Class|VisualLoggerKismetLibrary|LogText "About to create level" "Blueprint Log")
      (bind _returnvalue (Game|SpawnActorfromClass (Utilities|Array|Get(acopy) LevelList (+ (* _index MapTileCountX) _index_2)) (Math|Transform|MakeTransform (Math|Vector|MakeVector (- (* (- _index (/ MapTileCountX 2)) _sublevelsize) 2e+03) (* (- _index_2 (/ MapTileCountY 2)) _sublevelsize) -2.0) (Math|Conversions|RotationFromXVector (Math|Vector|MakeVector 0.0 (* (Math|Random|RandomInteger 3) 9e+01) 0.0))) "Undefined" 0 0))
      (if (!= _returnvalue 0)
        (Class|VisualLoggerKismetLibrary|LogText "level created" "Blueprint Log")
        (else
          (Class|VisualLoggerKismetLibrary|LogText (Utilities|String|Append "Could not create level with index " (Utilities|String|ToString(Float) (Variables|Default|GetSublevelSize))) "Blueprint Log"))))))

(event EventGenerateLevel
  (params (SubLevels :type Array%20of%20Names) (MapTileCountX :type Integer) (MapTileCountY :type Integer))
  (bind _sublevelsize (Variables|Default|GetSublevelSize))
  (Class|VisualLoggerKismetLibrary|LogText "Executing generate level.." "Blueprint Log")
  (for _index (range 0 MapTileCountX)
    (for _index_2 (range 0 MapTileCountY)
      (Class|VisualLoggerKismetLibrary|LogText "About to create level" "Blueprint Log")
      (bind _returnvalue (Class|LevelStreaming|CreateInstance (Class|GameplayStatics|GetStreamingLevel (Utilities|Array|Get(acopy) SubLevels (+ (* _index MapTileCountX) _index_2))) (Utilities|String|Append "level" (Utilities|String|ToString(Integer) _index) "x" (Utilities|String|ToString(Integer) _index_2))))
      (if (!= _returnvalue 0)
        (Class|VisualLoggerKismetLibrary|LogText "level created" "Blueprint Log")
        (else
          (Class|VisualLoggerKismetLibrary|LogText (Utilities|String|Append "Could not create level with index " (Utilities|String|ToString(Float) (Variables|Default|GetSublevelSize))) "Blueprint Log")))
      (Variables|/Script/Engine.LevelStreaming|SetLevelTransform _returnvalue (Math|Transform|MakeTransform (Math|Vector|MakeVector (* (- _index (/ MapTileCountX 2)) _sublevelsize) (* (- _index_2 (/ MapTileCountY 2)) _sublevelsize) -2.0) (Math|Conversions|RotationFromXVector (Math|Vector|MakeVector 0.0 (* (Math|Random|RandomInteger 3) 9e+01) 0.0))))
      (Class|VisualLoggerKismetLibrary|LogText "set level transform!" "Blueprint Log")
      (Variables|/Script/Engine.LevelStreaming|SetbShouldBeLoaded _returnvalue true)
      (Class|VisualLoggerKismetLibrary|LogText "Set should be loaded!" "Blueprint Log")
      (Variables|/Script/Engine.LevelStreaming|SetbShouldBeVisible _returnvalue true)
      (Class|VisualLoggerKismetLibrary|LogText "Set should be visible!" "Blueprint Log")
      (Variables|/Script/Engine.LevelStreaming|SetbShouldBlockOnLoad _returnvalue true))))

(fn ConstructionScript)